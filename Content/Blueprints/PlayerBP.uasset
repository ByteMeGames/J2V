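; Player character Blueprint for side-on movement along the world X axis, with jump, wall jump and dash.
; Jumping while falling runs a horizontal line trace from behind to ahead of the capsule at Y=0; a hit launches the character up and away from it, otherwise it calls Jump.
; Dash launches along X by scaling current velocity, more strongly on the ground than in the air, and zeroes vertical speed.
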(event `InputAxis|Move`
  (params (AxisValue :type "Float (single-precision)"))
  ;[1 1 1] Movement Control
  (`self.AddMovementInput` (1.0 0.0 0.0) AxisValue))

(event `InputAction|Jump`
  (params (Key :type "Key Structure" :default "AnyKey"))
  ;[1 1 1] Jumping
  (:`Pressed`
    (if (`NavMovementComponent.IsFalling` (`self.CharacterMovement`))
      (bind (_start _end) (`self.CalculateAroundPosition`))
      (`self.WallJump` _start _end)
      (else
        (`self.Jump`))))
  (:`Released`
    (`self.StopJumping`)))

(event `WallJump`
  (params (Start :type "Vector Structure") (End :type "Vector Structure"))
  (bind _returnvalue_x (`KismetMathLibrary.BreakVector` (`self.K2_GetActorLocation`)))
  (bind _jumpzvelocity (`CharacterMovementComponent.JumpZVelocity` (`self.CharacterMovement`)))
  ;[1 1 1] Wall Jump
  (bind (_outhit _returnvalue) (`KismetSystemLibrary.LineTraceSingle` Start End "TraceTypeQuery1" true))
  (if _returnvalue
    (`self.LaunchCharacter` (`KismetMathLibrary.MakeVector` (* (`KismetMathLibrary.SignOfFloat` (- _returnvalue_x (.x (`.Location` (`GameplayStatics.BreakHitResult` _outhit))))) _jumpzvelocity) 0.0 _jumpzvelocity) true true)
    (else
      (`self.Jump`))))

(event `InputAction|Dash`
  (params (Key :type "Key Structure" :default "AnyKey"))
  (bind _returnvalue (`self.GetVelocity`))
  ;[1 1 1] Dash
  (:`Pressed`
    (if (`NavMovementComponent.IsFalling` (`self.CharacterMovement`))
      (`self.LaunchCharacter` (* _returnvalue (1.8 0.0 0.0)) true true)
      (else
        (`self.LaunchCharacter` (* _returnvalue (5.0 0.0 0.0)) true true)))))

(fn `CalculateAroundPosition`
  (returns (start :type "Vector Structure") (end :type "Vector Structure"))
  (bind _returnvalue (* (`self.GetActorForwardVector`) (* (`CapsuleComponent.GetScaledCapsuleRadius` (`self.CapsuleComponent`)) 5.0)))
  (bind (_returnvalue_x _returnvalue_y _returnvalue_z) (`KismetMathLibrary.BreakVector` (- (`self.K2_GetActorLocation`) _returnvalue)))
  (bind (_returnvalue_x_2 _returnvalue_y_2 _returnvalue_z_2) (`KismetMathLibrary.BreakVector` (+ _returnvalue (`self.K2_GetActorLocation`))))
  (return (`KismetMathLibrary.MakeVector` _returnvalue_x 0.0 _returnvalue_z) (`KismetMathLibrary.MakeVector` _returnvalue_x_2 0.0 _returnvalue_z_2)))

(fn `UserConstructionScript`)