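; ParallaxBP is a parallax Blueprint that scrolls a Background component along X as the player character moves.
; BeginPlay caches player 0's character and stores InitialX as its world X plus the Background's relative X.
; Every Tick sets the Background's relative X to InitialX minus the player's current X, times ScrollScale, so the starting offset is scaled too.
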(event `self.ReceiveBeginPlay`
  (bind _relativelocation_x (`KismetMathLibrary.BreakVector` (`SceneComponent.RelativeLocation` (`self.Background`))))
  ;[1 1 1] Init
  (bind _output_get (set `self.CurrentPlayerCharacter` (`GameplayStatics.GetPlayerCharacter` 0)))
  (bind _returnvalue_x (`KismetMathLibrary.BreakVector` (`self.K2_GetActorLocation` _output_get)))
  (set `self.InitialX` (+ _returnvalue_x _relativelocation_x)))

(event `self.ReceiveTick`
  (params (DeltaSeconds :type "Float (single-precision)"))
  (bind _returnvalue_x (`KismetMathLibrary.BreakVector` (`self.K2_GetActorLocation` (`self.CurrentPlayerCharacter`))))
  ;[1 1 1] Parallax Scrolling
  (`SceneComponent.K2_SetRelativeLocation` (`self.Background`) (`KismetMathLibrary.MakeVector` (* (- (`self.InitialX`) _returnvalue_x) (`self.ScrollScale`))) false false))

(fn `UserConstructionScript`)